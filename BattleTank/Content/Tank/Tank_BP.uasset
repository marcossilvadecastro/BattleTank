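; Player-controllable tank pawn that drives on two tracks, aims and fires.
; On BeginPlay it wires barrel and turret into TankAiming, both tracks into TankMoviment, and itself into the health bar widget.
; Input drives each track directly or goes through the movement component, while frame-time-scaled axes rotate the azimuth gimbal and spring arm for camera aim.
; Swap Cam calls ToggleActive twice on the same third-person component.
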(event EventBeginPlay
  (Class|TankAimingComponent|Initialize (Variables|Default|GetTankAiming) (Variables|Default|GetBarrel) (Variables|Default|GetTankTurret))
  (Class|TankMovimentComponent|Initialize (Variables|Default|GetTankMoviment) (Variables|Default|GetLeft%20Track) (Variables|Default|GetRight%20Track))
  (CallFunction|InitializeHealth))

(event Input|ActionEvents|InputActionFire
  (params (Key :type Key%20Structure :default "AnyKey"))
  (:Pressed
    (Class|TankAimingComponent|Fire (Variables|Default|GetTankAiming))))

(event Input|ActionEvents|InputActionSwapCam
  (params (Key :type Key%20Structure :default "AnyKey"))
  (:Pressed
    (Components|Activation|ToggleActive (Variables|Default|Get3st%20person))
    (Components|Activation|ToggleActive (Variables|Default|Get3st%20person))))

(event Input|AxisEvents|InputAxisTurnRight
  (params (AxisValue :type Float%20%28single-precision%29))
  ;[1 1 1] Input Binding
  (Class|TankMovimentComponent|IntentMoveRight (Variables|Default|GetTankMoviment) AxisValue))

(event Input|AxisEvents|InputAxisAimElevation
  (params (AxisValue :type Float%20%28single-precision%29))
  ;[1 1 1] Camera Input Binding
  (Transformation|AddLocalRotation (Variables|Default|GetSpringArm) (Math|Rotator|MakeRotator 0.0 (* AxisValue (Utilities|Time|GetWorldDeltaSeconds) 1e+02) 0.0) false false))

(event Input|AxisEvents|InputAxisLeftTrackThrottle
  (params (AxisValue :type Float%20%28single-precision%29))
  ;[1 1 1] Input Binding
  (Class|TankTrack|SetThrottle (Variables|Default|GetLeft%20Track) AxisValue))

(event Input|AxisEvents|InputAxisMoveForward
  (params (AxisValue :type Float%20%28single-precision%29))
  ;[1 1 1] Input Binding
  (Class|TankMovimentComponent|MoveForward (Variables|Default|GetTankMoviment) AxisValue))

(event Input|AxisEvents|InputAxisRightTrackThrottle
  (params (AxisValue :type Float%20%28single-precision%29))
  ;[1 1 1] Input Binding
  (Class|TankTrack|SetThrottle (Variables|Default|GetRight%20Track) AxisValue))

(event Input|AxisEvents|InputAxisAimAzimuth
  (params (AxisValue :type Float%20%28single-precision%29))
  ;[1 1 1] Camera Input Binding
  (Transformation|AddLocalRotation (Variables|Default|GetAzimuth%20Gimbal) (Math|Rotator|MakeRotator 0.0 0.0 (* AxisValue (Utilities|Time|GetWorldDeltaSeconds) 1e+02)) false false))

(fn ConstructionScript)

(fn InitializeHealth
  (bind _asbar_health (Utilities|Casting|CastToBarHealth (UserInterface|GetUserWidgetObject (Variables|Default|GetWidgetHealth))))
  (Variables|/Game/UI/BarHealth.BarHealth_C|SetMyTank _asbar_health self)
  (return))